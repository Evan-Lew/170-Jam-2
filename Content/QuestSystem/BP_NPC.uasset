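; BP_NPC is a quest NPC that the player interacts with to advance a "find manager" objective.
; On BeginPlay it enables input, caches the BP_Quest_FindManager actor and adds a QuestManager widget to the viewport.
; Box overlap shows or hides a widget and opens or closes a Gate on the Interact input.
; While the gate is open, each press increases objective 0 on the quest actor and prints "Found Manager".
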(event `self.ReceiveBeginPlay`
  (`self.EnableInput` (`GameplayStatics.GetPlayerController` 0))
  (bind _returnvalue (`GameplayStatics.GetActorOfClass` "/Game/QuestSystem/BP_Quest_FindManager.BP_Quest_FindManager_C"))
  (set `self.ManagerQuest` _returnvalue)
  (`GameplayStatics.GetActorOfClass` "/Game/FirstPerson/Blueprints/BP_FirstPersonCharacter.BP_FirstPersonCharacter_C")
  (bind _returnvalue_2 (`|CreateWidget` "/Game/QuestSystem/QuestManager.QuestManager_C"))
  (`UserWidget.AddToViewport` _returnvalue_2 0))

(event `InputAction|Interact`
  (params (Key :type "Key Structure"))
  (:`Pressed`
    (`/Engine/EditorBlueprintResources/StandardMacros.Gate` true :!label _label
      (:`Exit`
        (`/Game/QuestSystem/BP_Quest.IncreaseObjectiveQuantity` (`self.ManagerQuest`) 0)
        (`KismetSystemLibrary.PrintText` "Found Manager")))))

(event `self.Box.OnComponentBeginOverlap`
  (params (OverlappedComponent :type "PrimitiveComponent Object Reference") (OtherActor :type "Actor Object Reference") (OtherComp :type "PrimitiveComponent Object Reference") (OtherBodyIndex :type Integer) (bFromSweep :type Boolean) (SweepResult :type "HitResult Structure (by ref)"))
  (`SceneComponent.SetHiddenInGame` (`self.Widget`) false false)
  (goto _label :!via `Open`))

(event `self.Box.OnComponentEndOverlap`
  (params (OverlappedComponent :type "PrimitiveComponent Object Reference") (OtherActor :type "Actor Object Reference") (OtherComp :type "PrimitiveComponent Object Reference") (OtherBodyIndex :type Integer))
  (`SceneComponent.SetHiddenInGame` (`self.Widget`) true false)
  (goto _label :!via `Close`))

(fn `UserConstructionScript`)