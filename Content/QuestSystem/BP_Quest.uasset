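; BP_Quest is a quest Blueprint that tracks a set of objectives and its own completed state.
; On BeginPlay it constructs an O_Objective for each ObjectivesList entry, binds its completion event and stores it.
; IncreaseObjectiveQuantity advances an objective by index, and completions increment a counter.
; SetAsCompleted flags the quest and fires OnCompleted, but the all-objectives-done check leads nowhere and never calls it.
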(event `self.ReceiveBeginPlay`
  (for _array_element (`self.ObjectivesList`)
    (bind (_title _quantitygoal) (break `/Game/QuestSystem/S_ObjectiveData` _array_element))
    (bind _returnvalue (`|GenericCreateObject` "/Game/QuestSystem/O_Objective.O_Objective_C" _title _quantitygoal))
    (add `/Game/QuestSystem/O_Objective.OnCompleted` _returnvalue (delegate `ObjectiveCompleted`))
    (`KismetArrayLibrary.Array_Add` (`self.ObjectiveData`) _returnvalue)))

(event `ObjectiveCompleted`
  (bind _completedobjectives (`self.CompletedObjectives`))
  (`/Engine/EditorBlueprintResources/StandardMacros.IncrementInt` _completedobjectives
    (:`  `
      (if (== (`KismetArrayLibrary.Array_Length` (`self.ObjectiveData`)) _completedobjectives)
        _))))

(fn `IncreaseObjectiveQuantity`
  (params (ObjectiveIndex :type Integer))
  (`/Game/QuestSystem/O_Objective.IncreaseQuantity` (`|GetArrayItem` (`self.ObjectiveData`) ObjectiveIndex)))

(fn `SetAsCompleted`
  (set `self.Completed` true)
  (`self.OnCompleted`))

(fn `UserConstructionScript`)